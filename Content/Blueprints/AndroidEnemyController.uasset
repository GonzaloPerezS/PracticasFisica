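; AI controller for an android enemy that detects the player through AI perception.
; It runs its behavior tree on possess.
; A successfully sensed Player-tagged actor clears the enemy timer, then, if perception is enabled, is written to the Blackboard with a target-detected flag.
; The file contains no logic for losing the target or starting that timer.
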(event `self.ReceivePossess`
  (params (PossessedPawn :type "Pawn Object Reference"))
  (`self.RunBehaviorTree` (`self.BTAsset`)))

(event `self.AIPerception.OnTargetPerceptionUpdated`
  (params (Actor :type "Actor Object Reference") (Stimulus :type "AIStimulus Structure"))
  (if (and (`self.ActorHasTag` Actor "Player") (`.bSuccessfullySensed` (break `AIStimulus` Stimulus)))
    (`KismetSystemLibrary.K2_ClearAndInvalidateTimerHandle` (`self.EnemyTimer`))
    (`self.DetectPlayer` Actor)))

(fn `DetectPlayer`
  (params (PlayerActor :type "Object Object Reference"))
  (bind _blackboard (`self.Blackboard`))
  (if (`self.PerceptionEnabled`)
    (`BlackboardComponent.SetValueAsBool` _blackboard (`self.IsTargetDetected`) true)
    (`BlackboardComponent.SetValueAsObject` _blackboard (`self.PlayerActor`) PlayerActor)))

(fn `UserConstructionScript`)