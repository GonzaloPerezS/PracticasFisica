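; Spawner actor that repeatedly spawns instances of a configurable class at random points inside a box, which the construction script sizes from Extent and raises above the origin.
; A DoOnce-gated loop, entered from StartSpawning or Tick, waits SpawnRatio seconds after each successful spawn and continues while Enabled.
; Failed collision-checked spawns retry immediately without a delay.
; StopSawning clears Enabled and resets the gate.
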(event `StartSpawning`
  (bind _returnvalue (* (`self.Extent`) 100.0))
  (set `self.bEnabled` true)
  (`/Engine/EditorBlueprintResources/StandardMacros.DoOnce` false :!label _label
    (:`Completed`
      (bind _returnvalue_2 (`|SpawnActorFromClass` (`self.ActorClass`) (`KismetMathLibrary.MakeTransform` (`KismetMathLibrary.RandomPointInBoundingBox` (+ (`self.K2_GetActorLocation`) (`KismetMathLibrary.MakeVector` 0.0 0.0 (.z _returnvalue))) _returnvalue) (struct :`Pitch` 90.0)) "AdjustIfPossibleButDontSpawnIfColliding" "MultiplyWithRoot" null null :!label _label_2))
      (`/Engine/EditorBlueprintResources/StandardMacros.IsValid` _returnvalue_2
        (:`Is Valid`
          (`KismetSystemLibrary.Delay` (`self.SpawnRatio`))
          (if (`self.bEnabled`)
            (goto _label_2)))
        (:`Is Not Valid`
          (goto _label_2))))))

(event `StopSawning`
  (set `self.bEnabled` false)
  (goto _label :!via `Reset`))

(event `self.ReceiveTick`
  (params (DeltaSeconds :type "Float (single-precision)"))
  (`/Engine/EditorBlueprintResources/StandardMacros.DoOnce` (not (`self.bEnabled`))
    (:`Completed`
      (goto _label_2))))

(fn `UserConstructionScript`
  (bind _box (`self.Box`))
  (bind _returnvalue (* (`self.Extent`) 100.0))
  (`BoxComponent.SetBoxExtent` _box _returnvalue true)
  (`SceneComponent.K2_SetRelativeLocation` _box (`KismetMathLibrary.MakeVector` 0.0 0.0 (.z _returnvalue)) false false))