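; BP_Grenade is a projectile actor that plays an explosion effect when it hits something.
; On hit, it turns off physics and collision on its collision component, hides its sphere, stops the projectile movement and activates the explosion particle system.
; BeginPlay binds the particle system's finished event, so the actor destroys itself once the effect completes.
; The Blueprint itself applies no damage.
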(event `self.ReceiveBeginPlay`
  (add `ParticleSystemComponent.OnSystemFinished` (`self.ExplosionPS`) (delegate `Destroy`)))

(event `Destroy`
  (params (PSystem :type "ParticleSystemComponent Object Reference"))
  (`self.K2_DestroyActor`))

(event `self.ReceiveHit`
  (params (MyComp :type "PrimitiveComponent Object Reference") (Other :type "Actor Object Reference") (OtherComp :type "PrimitiveComponent Object Reference") (bSelfMoved :type Boolean) (HitLocation :type "Vector Structure") (HitNormal :type "Vector Structure") (NormalImpulse :type "Vector Structure") (Hit :type "HitResult Structure (by ref)"))
  (`PrimitiveComponent.SetSimulatePhysics` (`self.CollisionComp`) false)
  (`PrimitiveComponent.SetCollisionEnabled` (`self.CollisionComp`) "NoCollision")
  (`ActorComponent.Activate` (`self.ExplosionPS`) false)
  (`SceneComponent.SetVisibility` (`self.Sphere`) false false)
  (`MovementComponent.StopMovementImmediately` (`self.ProjectileMovement`)))

(fn `UserConstructionScript`)